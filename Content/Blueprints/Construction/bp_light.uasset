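; Light Blueprint that blinks its point light on and off a limited number of times once play begins.
; BeginPlay branches on a Visibility flag, toggles the light through SwitchTheLight, waits the on or off delay, then flips the flag.
; A DoN node feeds back into the branch, so LightSwitchCounter caps how often the cycle repeats.
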(event `self.ReceiveBeginPlay`
  (if (`self.visibility`) :!label _label
    (`self.switch the light`)
    (`KismetSystemLibrary.Delay` (`self.delay light on`))
    (set `self.visibility` false)
    (else
      (`self.switch the light`)
      (`KismetSystemLibrary.Delay` (`self.delay light off`))
      (set `self.visibility` true)))
  (`/Engine/EditorBlueprintResources/StandardMacros.Do N` (`self.light switch counter`)
    (:`Exit`
      (goto _label))))

(fn `switch the light`
  (`SceneComponent.ToggleVisibility` (`self.PointLight`) false))

(fn `UserConstructionScript`)